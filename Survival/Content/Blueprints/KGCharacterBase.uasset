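; KGCharacterBase is the base knight character for player and AI, with sword melee, projectile magic and health.
; BeginPlay attaches a sword and binds a victory montage to the game mode's end dispatcher; construction sets hair colour and links the health bar.
; Melee chains combos through montage sections, and flinching blocks attacks.
; Damage triggers flinches or death, which ends the game for players and destroys AI knights after the animation.
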(event `self.ReceiveBeginPlay`
  (`self.CreateSword`)
  (bind _askggame_mode (cast `/Game/Blueprints/KGGameMode` (`GameplayStatics.GetGameMode`)))
  (add `/Game/Blueprints/KGGameMode.EndGameDispatcher` _askggame_mode (delegate `EndGameDance`)))

(event `EndGameDance`
  (if (> (`self.Health`) 0.0)
    (`CharacterMovementComponent.DisableMovement` (`self.CharacterMovement`))
    (`|PlayMontage` null "/Game/Assets/Knight/VictoryMontage.VictoryMontage")))

(event `self.ReceiveAnyDamage`
  (params (Damage :type "Float (single-precision)") (DamageType :type "DamageType Object Reference") (InstigatedBy :type "Controller Object Reference") (DamageCauser :type "Actor Object Reference"))
  (bind _returnvalue (`SkeletalMeshComponent.GetAnimInstance` (`self.Mesh`)))
  (bind _output_get (set `self.Health` (- (`self.Health`) Damage)))
  (if (<= _output_get 0.0)
    (`/Engine/EditorBlueprintResources/StandardMacros.DoOnce` false
      (:`Completed`
        (set `self.IsFlinching` true)
        (`CharacterMovementComponent.DisableMovement` (`self.CharacterMovement`))
        (bind _returnvalue_2 (`self.PlayAnimMontage` "/Game/Assets/Knight/PlayerDeath.PlayerDeath"))
        (if (`Controller.IsPlayerController` (`self.GetController`))
          (`/Game/Blueprints/KGGameMode.EndGame` (cast `/Game/Blueprints/KGGameMode` (`GameplayStatics.GetGameMode`) :!pure true))
          (else
            (`KismetSystemLibrary.Delay` _returnvalue_2)
            (`self.K2_DestroyActor` (`self.Sword`))
            (`self.K2_DestroyActor`)))))
    (else
      (set `self.IsFlinching` true)
      (if (`AnimInstance.Montage_IsActive` _returnvalue "/Game/Assets/Knight/KnightAttackMontage.KnightAttackMontage")
        (if (`KismetArrayLibrary.Array_Contains` (`self.AttackMoves`) (`AnimInstance.Montage_GetCurrentSection` _returnvalue "/Game/Assets/Knight/KnightAttackMontage.KnightAttackMontage"))
          (set `self.IsFlinching` false)
          (else
            (bind _returnvalue_3 (`self.PlayAnimMontage` "/Game/Assets/Knight/PlayerFlinch.PlayerFlinch" 1.0 "FlinchBig"))
            (`KismetSystemLibrary.Delay` _returnvalue_3)
            (set `self.IsFlinching` false)))
        (else
          (bind _returnvalue_4 (`self.PlayAnimMontage` "/Game/Assets/Knight/PlayerFlinch.PlayerFlinch" 1.0 "FlinchSmall"))
          (`KismetSystemLibrary.Delay` _returnvalue_4)
          (set `self.IsFlinching` false))))))

(event `TryMelee`
  (bind _returnvalue (`SkeletalMeshComponent.GetAnimInstance` (`self.Mesh`)))
  (bind _returnvalue_2 (`AnimInstance.Montage_GetCurrentSection` _returnvalue "/Game/Assets/Knight/KnightAttackMontage.KnightAttackMontage"))
  (if (`self.IsFlinching`)
    _
    (elif (`AnimInstance.Montage_IsActive` _returnvalue "/Game/Assets/Knight/KnightAttackMontage.KnightAttackMontage")
      (switch `name` _returnvalue_2
        (:`Attack1`
          (`AnimInstance.Montage_SetNextSection` _returnvalue _returnvalue_2 "Attack2" "/Game/Assets/Knight/KnightAttackMontage.KnightAttackMontage")))
      (else
        (`self.PlayAnimMontage` "/Game/Assets/Knight/KnightAttackMontage.KnightAttackMontage" 1.0 "Attack1")))))

(event `TryMagic`
  (if (not (`self.IsFlinching`))
    (`self.PlayAnimMontage` "/Game/Assets/Knight/MagicShootMontage.MagicShootMontage")))

(event `CreateSword`
  (bind _returnvalue (`|SpawnActorFromClass` "/Game/Blueprints/BaseSword.BaseSword_C" (`self.GetTransform`) "Undefined" "OverrideRootScale"))
  (bind _output_get (set `self.Sword` _returnvalue))
  (`self.K2_AttachToComponent` _returnvalue (`self.Mesh`) "Sword" "SnapToTarget" "SnapToTarget" "SnapToTarget" false)
  (`self.K2_AttachToComponent` _output_get (`self.Mesh`) "Sword" "SnapToTarget" "SnapToTarget" "SnapToTarget" false))

(event `LaunchMagicProjectile`
  (`|SpawnActorFromClass` "/Game/Blueprints/KGProjectileBase.KGProjectileBase_C" (`SceneComponent.K2_GetComponentToWorld` (`self.Arrow1`)) "Undefined" "OverrideRootScale" null self))

(event `UsePrimaryAttack`
  (`self.TryMelee`))

(fn `UserConstructionScript`
  (bind _returnvalue (`PrimitiveComponent.CreateDynamicMaterialInstance` (`self.Mesh`) 0 null))
  (`MaterialInstanceDynamic.SetVectorParameterValue` _returnvalue "HairColour" (`self.HairColour`))
  (bind _asuihealth_bar (cast `/Game/Blueprints/UIHealthBar` (`WidgetComponent.GetUserWidgetObject` (`self.HealthBar`))))
  (`/Game/Blueprints/UIHealthBar.SetOwningKnightCharacter` _asuihealth_bar self))